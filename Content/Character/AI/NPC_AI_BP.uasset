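; NPC_AI_BP is an AI controller for guard NPCs that runs their behavior tree and tracks perceived targets.
; On begin play it sets up the PatrolData blackboard and starts the GuardBehaviour tree.
; AI perception updates write any sensed actor without the "Enemy" tag to the blackboard's enemy key.
; The key clears when such an actor's stimulus is lost, while actors tagged "Enemy" are ignored.
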(event `self.ReceiveBeginPlay`
  ;[1 1 1] Set Blackboard and Behaviour Tree
  (bind _blackboardcomponent (`self.UseBlackboard` "/Game/Character/AI/PatrolData.PatrolData"))
  (set `self.BlackboardComp` _blackboardcomponent)
  (`self.RunBehaviorTree` "/Game/Character/AI/GuardBehaviour.GuardBehaviour"))

(event `self.AIPerception.OnTargetPerceptionUpdated`
  (params (Actor :type "Actor Object Reference") (Stimulus :type "AIStimulus Structure"))
  (bind _blackboardcomp (`self.BlackboardComp`))
  (bind _enemykey (`self.EnemyKey`))
  ;[1 1 1] Enemy Detected
  (`/Engine/EditorBlueprintResources/StandardMacros.IsValid` Actor
    (:`Is Valid`
      (if (`self.ActorHasTag` Actor "Enemy")
        _
        (elif (`.bSuccessfullySensed` (break `AIStimulus` Stimulus))
          (`BlackboardComponent.SetValueAsObject` _blackboardcomp _enemykey Actor)
          (else
            (`BlackboardComponent.ClearValue` _blackboardcomp _enemykey)))))))

(fn `UserConstructionScript`)