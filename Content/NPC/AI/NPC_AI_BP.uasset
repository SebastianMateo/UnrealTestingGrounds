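; AI controller for an NPC guard that sets up the PatrolData blackboard and runs the GuardBehaviour tree on BeginPlay.
; AI perception updates respond only to actors without the "Enemy" tag.
; A sensed actor becomes the EnemyKey blackboard value and switches the controlled TP_Character to aiming and shooting.
; Losing the stimulus clears the key and aiming but still sets Shooting to true.
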(event `self.ReceiveBeginPlay`
  (bind _blackboardcomponent (`self.UseBlackboard` "/Game/NPC/AI/PatrolData.PatrolData"))
  (set `self.BlackboardComp` _blackboardcomponent)
  (`self.RunBehaviorTree` "/Game/NPC/AI/GuardBehaviour.GuardBehaviour"))

(event `self.AIPerception.OnTargetPerceptionUpdated`
  (params (Actor :type "Actor Object Reference") (Stimulus :type "AIStimulus Structure"))
  (bind _returnvalue (`self.K2_GetPawn`))
  (bind _blackboardcomp (`self.BlackboardComp`))
  (bind _enemykey (`self.EnemyKey`))
  (if (`self.ActorHasTag` Actor "Enemy")
    _
    (elif (`.bSuccessfullySensed` (break `AIStimulus` Stimulus))
      (bind _astp_character (cast `/Game/NPC/Behaviour/TP_Character` _returnvalue))
      (set `/Game/NPC/Behaviour/TP_Character.Aiming` true _astp_character)
      (set `/Game/NPC/Behaviour/TP_Character.Shooting` true _astp_character)
      (`BlackboardComponent.SetValueAsObject` _blackboardcomp _enemykey Actor)
      (else
        (bind _astp_character_2 (cast `/Game/NPC/Behaviour/TP_Character` _returnvalue))
        (set `/Game/NPC/Behaviour/TP_Character.Aiming` false _astp_character_2)
        (set `/Game/NPC/Behaviour/TP_Character.Shooting` true _astp_character_2)
        (`BlackboardComponent.ClearValue` _blackboardcomp _enemykey)))))

(fn `UserConstructionScript`)